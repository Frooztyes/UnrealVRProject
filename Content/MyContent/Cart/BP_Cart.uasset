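; BP_Cart is a cart that finds rails beneath it and grinds along their splines.
; While off-rail, Tick sphere-traces downward and queries hit actors through grind messages for spline, start point, direction and offset.
; Grinding disables physics, starts a MoveComponentTo snap, then advances spline distance each tick with interpolated rotation.
; Closed loops wrap around, while open rail ends restore physics and briefly pause detection.
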(event `self.ReceiveBeginPlay`
  (set `self.canDetect` true))

(event `self.ReceiveTick`
  (params (DeltaSeconds :type "Float (single-precision)"))
  (bind _rail_point (`self.rail point`))
  (bind _rail_point_2 (`self.rail point`))
  (bind _rail_spline (`self.rail spline`))
  (bind (_returnvalue_roll _returnvalue_pitch _returnvalue_yaw) (`KismetMathLibrary.BreakRotator` (`SplineComponent.GetRotationAtDistanceAlongSpline` _rail_spline _rail_point_2 "World")))
  (bind _returnvalue (> (`self.rail direction`) 0.0))
  (bind _returnvalue_2 (+ (`self.K2_GetActorLocation`) (0.0 0.0 -50.0)))
  (if (`self.is on rail`)
    (`/Engine/EditorBlueprintResources/StandardMacros.IsValid` (`self.rail spline`)
      (:`Is Valid`
        (set `self.rail point` (+ (* DeltaSeconds (`self.movespeed`) (`self.rail direction`)) _rail_point_2))
        (if (or (> _rail_point (`SplineComponent.GetSplineLength` (`self.rail spline`))) (< _rail_point 0.0))
          (if (`SplineComponent.IsClosedLoop` (`self.rail spline`))
            (set `self.rail point` (`KismetMathLibrary.SelectFloat` (- (`SplineComponent.GetSplineLength` (`self.rail spline`)) 1.0) 0.0 (< (`self.rail point`) 0.0)))
            (else
              (`PrimitiveComponent.SetSimulatePhysics` (`self.Cart`) true)
              (set `self.is on rail` false)
              (set `self.rail spline` null)
              (`PrimitiveComponent.AddImpulse` (`self.Cart`) (0.0 0.0 0.0) "None" true)
              (set `self.canDetect` false)
              (`KismetSystemLibrary.Delay` 0.0)
              (set `self.canDetect` true)))
          (else
            (`self.K2_SetActorLocationAndRotation` (+ (`SplineComponent.GetLocationAtDistanceAlongSpline` _rail_spline _rail_point_2 "World") (`KismetMathLibrary.MakeVector` 0.0 0.0 (`self.rail offset`))) (`KismetMathLibrary.RInterpTo` (`self.K2_GetActorRotation`) (`KismetMathLibrary.MakeRotator` (* (`KismetMathLibrary.SelectFloat` 1.0 -1.0 _returnvalue) _returnvalue_pitch) (* _returnvalue_roll (`KismetMathLibrary.SelectFloat` -1.0 1.0 _returnvalue)) (+ _returnvalue_yaw (`KismetMathLibrary.SelectFloat` 0.0 180.0 _returnvalue) 90.0)) (`GameplayStatics.GetWorldDeltaSeconds`)))
            (set `self.movespeed` (`self.defaultMoveSpeed`)))))
      (:`Is Not Valid`))
    (elif (`self.canDetect`)
      (bind (_outhit _returnvalue_3) (`KismetSystemLibrary.SphereTraceSingle` :`Start` _returnvalue_2 :`End` (+ _returnvalue_2 (* (`self.GetActorUpVector`) -200.0)) :`Radius` 40.0 :`TraceChannel` "TraceTypeQuery2" :`DrawDebugType` "ForOneFrame"))
      (if _returnvalue_3
        (bind (_bblockinghit _binitialoverlap _time _distance _location _impactpoint _normal _impactnormal _physmat _hitactor) (`GameplayStatics.BreakHitResult` _outhit))
        (bind _yes (message `/Game/MyContent/BPI_Grindable.CanGrind?` _hitactor))
        (if _yes
          (bind (_grind_splite _start_point _direction _grind_offset) (message `/Game/MyContent/BPI_Grindable.GetGrindSpline` _hitactor _location (`self.K2_GetActorLocation`) (`KismetMathLibrary.VSize` (`self.GetVelocity`))))
          (set `self.rail spline` _grind_splite)
          (set `self.rail point` _start_point)
          (set `self.rail direction` _direction)
          (set `self.rail offset` _grind_offset)))
      (`/Engine/EditorBlueprintResources/StandardMacros.IsValid` (`self.rail spline`)
        (:`Is Valid`
          (`self.Start Grinding`))))))

(event `Start Grinding`
  (bind (_returnvalue_roll _returnvalue_pitch _returnvalue_yaw) (`KismetMathLibrary.BreakRotator` (`SplineComponent.GetRotationAtDistanceAlongSpline` (`self.rail spline`) (`self.rail point`) "World")))
  (bind _returnvalue (+ (`SplineComponent.GetLocationAtDistanceAlongSpline` (`self.rail spline`) (`self.rail point`) "World") (`KismetMathLibrary.MakeVector` 0.0 0.0 (`self.rail offset`))))
  (`PrimitiveComponent.SetSimulatePhysics` (`self.Cart`) false)
  (set `self.movespeed` (`self.defaultMoveSpeed`))
  (`KismetSystemLibrary.MoveComponentTo` (`self.Cart`) _returnvalue (`KismetMathLibrary.MakeRotator` 0.0 0.0 (+ (+ _returnvalue_yaw (`KismetMathLibrary.SelectFloat` 0.0 180.0 (> (`self.rail direction`) 0.0))) 90.0)) false false (/ (`KismetMathLibrary.Vector_Distance` _returnvalue (`SceneComponent.K2_GetComponentLocation` (`self.Cart`))) (`self.movespeed`)))
  (set `self.is on rail` true))

(fn `GetPlayerPosition`
  (returns (position :type "Vector Structure"))
  (return (`SceneComponent.K2_GetComponentLocation` (`self.PlayerPosition`))))

(fn `SetSpeed`
  (params (`new speed` :type "Float (double-precision)"))
  (set `self.defaultMoveSpeed` `new speed`))

(fn `UserConstructionScript`)