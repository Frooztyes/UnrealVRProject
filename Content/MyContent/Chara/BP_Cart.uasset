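; BP_Cart is a cart that rides along splines supplied by grindable actors beneath it.
; Each tick a downward debug-drawn sphere trace queries the hit actor through messages for spline, start point, direction and offset.
; With a valid spline, it eases the Cube onto that point and advances the actor at fixed speed, resetting distance to zero past either end.
; StopGrind, with skateboard physics, and a forward-angled detection variant are never called.
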(event `self.ReceiveBeginPlay`)

(event `self.ReceiveTick`
  (params (DeltaSeconds :type "Float (single-precision)"))
  (bind _grind_point (`self.grind point`))
  (bind _grind_spline (`self.grind spline`))
  (bind _grind_point_2 (`self.grind point`))
  (bind (_returnvalue_roll _returnvalue_pitch _returnvalue_yaw) (`KismetMathLibrary.BreakRotator` (`SplineComponent.GetRotationAtDistanceAlongSpline` _grind_spline _grind_point "World")))
  (bind _returnvalue (+ (`self.K2_GetActorLocation`) (0.0 0.0 -30.0)))
  (bind (_outhit _returnvalue_2) (`KismetSystemLibrary.SphereTraceSingle` :`Start` _returnvalue :`End` (+ _returnvalue (* (`self.GetActorUpVector`) -200.0)) :`Radius` 40.0 :`TraceChannel` "TraceTypeQuery2" :`DrawDebugType` "ForOneFrame"))
  (if _returnvalue_2
    (bind (_bblockinghit _binitialoverlap _time _distance _location _impactpoint _normal _impactnormal _physmat _hitactor) (`GameplayStatics.BreakHitResult` _outhit))
    (bind _yes (message `/Game/MyContent/BPI_Grindable.CanGrind?` _hitactor))
    (if _yes
      (bind (_grind_splite _start_point _direction _grind_offset) (message `/Game/MyContent/BPI_Grindable.GetGrindSpline` _hitactor _location (`self.K2_GetActorLocation`) (`KismetMathLibrary.VSize` (`self.GetVelocity`))))
      (set `self.grind spline` _grind_splite)
      (set `self.grind point` _start_point)
      (set `self.grind direction` _direction)
      (set `self.grind offset` _grind_offset)))
  (`/Engine/EditorBlueprintResources/StandardMacros.IsValid` (`self.grind spline`)
    (:`Is Valid`
      (`self.Start Grinding`)
      (`/Engine/EditorBlueprintResources/StandardMacros.IsValid` (`self.grind spline`)
        (:`Is Valid`
          (set `self.grind point` (+ (* DeltaSeconds (`self.movespeed`) (`self.grind direction`)) _grind_point))
          (if (or (> _grind_point_2 (`SplineComponent.GetSplineLength` (`self.grind spline`))) (< _grind_point_2 0.0))
            (set `self.grind point` 0.0)
            (else
              (`self.K2_SetActorLocationAndRotation` (+ (`SplineComponent.GetLocationAtDistanceAlongSpline` _grind_spline _grind_point "World") (0.0 0.0 96.0) (`KismetMathLibrary.MakeVector` 0.0 0.0 (`self.grind offset`))) (`KismetMathLibrary.MakeRotator` 0.0 0.0 (+ _returnvalue_yaw (`KismetMathLibrary.SelectFloat` 0.0 180.0 (> (`self.grind direction`) 0.0))))))))
        (:`Is Not Valid`)))))

(event `Start Grinding`
  (bind _grind_spline (`self.grind spline`))
  (bind _grind_point (`self.grind point`))
  (bind (_returnvalue_roll _returnvalue_pitch _returnvalue_yaw) (`KismetMathLibrary.BreakRotator` (`SplineComponent.GetRotationAtDistanceAlongSpline` _grind_spline _grind_point "World")))
  (bind _returnvalue (+ (`SplineComponent.GetLocationAtDistanceAlongSpline` _grind_spline _grind_point "World") (0.0 0.0 0.0) (`KismetMathLibrary.MakeVector` 0.0 0.0 (`self.grind offset`))))
  (set `self.movespeed` 500.0)
  (`KismetSystemLibrary.MoveComponentTo` (`self.Cube`) _returnvalue (`KismetMathLibrary.MakeRotator` 0.0 0.0 (+ (+ _returnvalue_yaw (`KismetMathLibrary.SelectFloat` 0.0 180.0 (> (`self.grind direction`) 0.0))) 90.0)) false false (/ (`KismetMathLibrary.Vector_Distance` _returnvalue (`SceneComponent.K2_GetComponentLocation` (`self.Cube`))) (`self.movespeed`))))

(fn `UserConstructionScript`)