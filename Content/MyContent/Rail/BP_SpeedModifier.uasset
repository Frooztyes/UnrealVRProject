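; BP_SpeedModifier is a rail trigger that changes the speed of the VR player's cart.
; On BeginPlay it caches the MyVRPawn player, and any overlap on its collision component sets that pawn's cart to MultiplierSpeed times its default move speed.
; A DoOnce blocks retriggering and reopens five seconds after a successful change; the speed itself is never restored here.
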(event `self.ReceiveTick`
  (params (DeltaSeconds :type "Float (single-precision)")))

(event `self.ReceiveBeginPlay`
  (bind _asmy_vrpawn (cast `/Game/VRTemplate/Blueprints/MyVRPawn` (`GameplayStatics.GetPlayerPawn` 0)))
  (set `self.player` _asmy_vrpawn))

(event `self.CollisionComponent.OnComponentBeginOverlap`
  (params (OverlappedComponent :type "PrimitiveComponent Object Reference") (OtherActor :type "Actor Object Reference") (OtherComp :type "PrimitiveComponent Object Reference") (OtherBodyIndex :type Integer) (bFromSweep :type Boolean) (SweepResult :type "HitResult Structure (by ref)"))
  (bind _cart (`/Game/VRTemplate/Blueprints/MyVRPawn.cart` (`self.player`)))
  (`/Engine/EditorBlueprintResources/StandardMacros.DoOnce` false :!label _label
    (:`Completed`
      (`/Engine/EditorBlueprintResources/StandardMacros.IsValid` _cart
        (:`Is Valid`
          (`/Game/MyContent/Cart/BP_Cart.SetSpeed` _cart (* (`self.multiplierSpeed`) (`/Game/MyContent/Cart/BP_Cart.defaultMoveSpeed` _cart)))
          (`KismetSystemLibrary.Delay` 5.0)
          (goto _label :!via `Reset`))))))

(fn `UserConstructionScript`)