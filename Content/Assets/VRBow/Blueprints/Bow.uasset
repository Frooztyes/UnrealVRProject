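; VR bow actor that snaps to the pawn's left grip controller and fires arrows drawn with the right hand.
; Grabbing with the right controller spawns an arrow; Tick then bends the two spline-mesh string halves to that hand and aims bow and arrow along the line between controllers.
; Release resets string and bow rotation, then fires the arrow with force scaled by hand separation.
; The construction script computes the string's rest midpoint from its end markers.
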(event `/Game/Assets/VRBow/Interface/Grab.Grab`
  (params (MotionController :type "MotionControllerComponent Object Reference"))
  (if (== MotionController (`self.SecondaryMotionController`))
    (set `self.is shooting` true)
    (`self.Arrow`
      (:`then`)
      (:`else`
        (bind _returnvalue (`|SpawnActorFromClass` "/Game/Assets/VRBow/Blueprints/Arrow.Arrow_C" (`KismetMathLibrary.MakeTransform` (0.0 0.0 0.0)) "AlwaysSpawn" "MultiplyWithRoot" null null))
        (bind _output_get (set `self.Arrow` _returnvalue))
        (set `/Game/Assets/VRBow/Blueprints/Arrow.Bow` self _output_get)
        (bind _asmy_vrpawn (cast `/Game/VRTemplate/Blueprints/MyVRPawn` (`GameplayStatics.GetPlayerPawn` 0)))
        (set `/Game/Assets/VRBow/Blueprints/Arrow.VRPawn` _asmy_vrpawn _output_get)))))

(event `self.ReceiveBeginPlay`
  (bind _asmy_vrpawn (cast `/Game/VRTemplate/Blueprints/MyVRPawn` (`GameplayStatics.GetPlayerPawn` 0)))
  (bind (_motioncontrollerrightgrip _motioncontrollerleftgrip) (`/Game/VRTemplate/Blueprints/MyVRPawn.GetMotionControllers` _asmy_vrpawn))
  (set `self.SecondaryMotionController` _motioncontrollerrightgrip)
  ;[0 0 0] Accrocher Arc Main Gauche
  (bind _output_get (set `self.PrimaryMotionController` _motioncontrollerleftgrip))
  (`self.K2_AttachToComponent` _output_get "None" "SnapToTarget" "SnapToTarget" "KeepWorld")
  (`self.K2_SetActorRelativeRotation` (struct :`Pitch` -90.0)))

(event `/Game/Assets/VRBow/Interface/Grab.Release`
  (params (MotionController :type "MotionControllerComponent Object Reference"))
  (if (== MotionController (`self.SecondaryMotionController`))
    (set `self.Multiplier` (* (`KismetMathLibrary.Vector_Distance` (`SceneComponent.K2_GetComponentLocation` (`self.PrimaryMotionController`)) (`SceneComponent.K2_GetComponentLocation` (`self.SecondaryMotionController`))) 10000.0))
    (`SplineMeshComponent.SetEndPosition` (`self.UpperString`) (`self.MidPoint`) true)
    (`SplineMeshComponent.SetEndPosition` (`self.DownString`) (`self.MidPoint`) true)
    (`self.K2_SetActorRelativeRotation` (struct :`Pitch` -90.0))
    (bind _arrow (`self.Arrow`)
      (:`then`
        (`/Game/Assets/VRBow/Blueprints/Arrow.Fire` _arrow (`self.Multiplier`))
        (set `self.Arrow` null)
        (set `self.is shooting` false))
      (:`else`))))

(event `self.ReceiveTick`
  (params (DeltaSeconds :type "Float (single-precision)"))
  (bind _returnvalue (`SceneComponent.K2_GetComponentLocation` (`self.SecondaryMotionController`)))
  (bind _returnvalue_2 (`KismetMathLibrary.FindLookAtRotation` _returnvalue (`SceneComponent.K2_GetComponentLocation` (`self.PrimaryMotionController`))))
  (if (`self.is shooting`)
    (bind _secondarymotioncontroller (`self.SecondaryMotionController`)
      (:`then`
        (bind (_returnvalue_x _returnvalue_y _returnvalue_z) (`KismetMathLibrary.BreakVector` (`KismetMathLibrary.InverseTransformLocation` (`SceneComponent.K2_GetComponentToWorld` (`self.DefaultSceneRoot`)) (`SceneComponent.K2_GetComponentLocation` _secondarymotioncontroller))))
        (`SplineMeshComponent.SetEndPosition` (`self.UpperString`) (`KismetMathLibrary.MakeVector` (- 0.0 _returnvalue_x) (- 0.0 _returnvalue_y) _returnvalue_z) true)
        (`SplineMeshComponent.SetEndPosition` (`self.DownString`) (`KismetMathLibrary.MakeVector` (- 0.0 _returnvalue_x) (- 0.0 _returnvalue_y) _returnvalue_z) true)
        (`self.K2_SetActorRotation` _returnvalue_2)
        (bind _arrow (`self.Arrow`)
          (:`then`
            (`self.K2_SetActorLocationAndRotation` _arrow _returnvalue _returnvalue_2 false false))
          (:`else`)))
      (:`else`))))

(fn `UserConstructionScript`
  (bind _scaledupposition (`self.ScaledUpPosition`))
  (bind _scaleddownposition (`self.ScaledDownPosition`))
  (set `self.ScaledUpPosition` (`SceneComponent.RelativeLocation` (`self.UpPosition`)))
  (set `self.ScaledDownPosition` (`SceneComponent.RelativeLocation` (`self.DownPosition`)))
  (bind _output_get (set `self.MidPoint` (+ _scaledupposition (* (/ (`KismetMathLibrary.Vector_Distance` _scaledupposition _scaleddownposition) 2.0) (`KismetMathLibrary.GetForwardVector` (`KismetMathLibrary.FindLookAtRotation` _scaledupposition _scaleddownposition))))))
  (`SplineMeshComponent.SetStartAndEnd` (`self.UpperString`) (`self.ScaledUpPosition`) (0.0 0.0 0.0) _output_get (0.0 0.0 0.0) true)
  (`SplineMeshComponent.SetStartAndEnd` (`self.DownString`) (`self.ScaledDownPosition`) (0.0 0.0 0.0) _output_get (0.0 0.0 0.0) true))