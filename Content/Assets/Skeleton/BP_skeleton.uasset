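; Skeleton enemy that wanders the navmesh and attacks the VR player when PawnSensing spots them.
; After a spawn delay it loops random moves; on sight it approaches the player's cart and plays an attack montage.
; During a timed attack window, Tick sphere-traces between two scene components, printing one hit per swing without applying damage.
; Kill halts movement, disables capsule collision and dims its light; CanAct gates behavior.
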(event `self.ReceiveBeginPlay`
  (`KismetSystemLibrary.Delay` 3.0)
  (set `self.is_spawning` false)
  (`self.MoveToRandomLocation`))

(event `MoveToRandomLocation`
  (`KismetSystemLibrary.Delay` 2.0)
  (if (`self.canAct`)
    (bind _randomlocation (`NavigationSystemV1.K2_GetRandomLocationInNavigableRadius` (`self.K2_GetActorLocation`) 1000.0 null null))
    (`|AIMoveTo` self _randomlocation null
      (:`OnSuccess`
        (`self.MoveToRandomLocation`)))))

(event `self.PawnSensing.OnSeePawn`
  (params (Pawn :type "Pawn Object Reference"))
  (if (`self.canAct`)
    (bind _asmy_vrpawn (cast `/Game/VRTemplate/Blueprints/MyVRPawn` Pawn))
    (`|AIMoveTo` self (0.0 0.0 0.0) (`/Game/VRTemplate/Blueprints/MyVRPawn.cart` _asmy_vrpawn) 200.0
      (:`OnSuccess`
        (`/Engine/EditorBlueprintResources/StandardMacros.DoOnce` false :!label _label
          (:`Completed`
            (`self.PlayAnimMontage` "/Game/Assets/Skeleton/skeleton_attack.skeleton_attack")
            (`KismetSystemLibrary.Delay` 1.0)
            (set `self.is_attacking` true)
            (`KismetSystemLibrary.Delay` 1.0)
            (set `self.is_attacking` false)
            (set `self.cannot_hit` false)
            (goto _label :!via `Reset`))))
      (:`OnFail`
        (`self.MoveToRandomLocation`)))))

(event `self.ReceiveTick`
  (params (DeltaSeconds :type "Float (single-precision)"))
  (if (`self.canAct`)
    (if (and (`self.is_attacking`) (not (`self.cannot_hit`)))
      (bind _outhits (`KismetSystemLibrary.SphereTraceMulti` (`SceneComponent.K2_GetComponentLocation` (`self.Scene1`)) (`SceneComponent.K2_GetComponentLocation` (`self.Scene`)) 100.0 "TraceTypeQuery2" true))
      (for _array_element _outhits
        (cast `/Game/VRTemplate/Blueprints/MyVRPawn` (`.HitActor` (`GameplayStatics.BreakHitResult` _array_element)))
        (set `self.cannot_hit` true)
        (`KismetSystemLibrary.PrintString` "Player hit")))))

(event `Kill`
  (bind _ominiouslight (`self.OminiousLight`))
  (set `self.is_dead` true)
  (`|AIMoveTo` self (`self.K2_GetActorLocation` self) null
    (:`then`
      (`PrimitiveComponent.SetCollisionEnabled` (`self.CapsuleComponent`) "NoCollision")
      (`LightComponent.SetIntensity` _ominiouslight (/ (`LightComponentBase.Intensity` _ominiouslight) 10.0)))))

(fn `setSightRange`
  (params (new_sight_range :type "Float (double-precision)"))
  (set `PawnSensingComponent.SightRadius` new_sight_range (`self.PawnSensing`)))

(fn `UserConstructionScript`)